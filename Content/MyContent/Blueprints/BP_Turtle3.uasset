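; BP_Turtle3 is a turtle actor that, once activated, travels along its SplinePath and disappears at the end.
; AccelerationTimeline1 drives position and rotation along the spline, while a looping timer with delays periodically reverses it briefly for a back-and-forth rhythm.
; AccelerationTimeline ramps the Speed variable, then reverses when the path finishes, ending in an emitter, sound and actor destruction.
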(event Custom|Rithm
  (bind _accelerationtimeline1 (Variables|Default|GetAccelerationTimeline1))
  (Utilities|FlowControl|Delay 1.0)
  (Utilities|String|Reverse _accelerationtimeline1)
  (Utilities|FlowControl|Delay 0.5)
  (Audio|Components|Audio|Play _accelerationtimeline1)
  (if (Variables|Default|GetShouldStop)
    (Utilities|Time|ClearandInvalidateTimerbyHandle (Variables|Default|GetRithmTimer))))

(event EventActivate
  (bind _returnvalue (Transformation|GetActorLocation))
  (bind _splinepath (Variables|Default|GetSplinePath))
  (bind _splinecomponent (Variables|/Game/MyContent/Blueprints/BP_SplinePath.BP_SplinePath_C|GetSplineComponent _splinepath))
  (Utilities|IsValid (Variables|Default|GetSplinePath)
    (:Is%20Valid
      (Components|Timeline|SetPlayRate (Variables|Default|GetAccelerationTimeline1) 0.2)
      (Utilities|FlowControl|Sequence
        (:then_0
          (bind _newtrack_0 (Timeline|AccelerationTimeline1 PlayFromStart)
            (:Update
              (Transformation|SetActorTransform (Math|Transform|MakeTransform (Spline|GetLocationatDistanceAlongSpline _splinecomponent (* (Spline|GetSplineLength _splinecomponent) _newtrack_0) "World") (Spline|GetRotationatDistanceAlongSpline _splinecomponent (* (Spline|GetSplineLength _splinecomponent) _newtrack_0) "Local") "1,1,1")))
            (:Finished
              (Variables|Default|SetShouldStop true)
              (Components|Timeline|ReversefromEnd (Variables|Default|GetAccelerationTimeline)))))
        (:then_1
          (bind (_direction _newtrack_0_2) (Timeline|AccelerationTimeline PlayFromStart)
            (:Update
              (Variables|Default|SetSpeed _newtrack_0_2))
            (:Finished
              (if (Utilities|Enum|Equal(Enum) _direction "Backward")
                (Effects|SpawnEmitteratLocation 0 _returnvalue "0, 0, 0" "2.000000,2.000000,2.000000")
                (Audio|PlaySoundatLocation "/Game/MyContent/Assets/Sounds/Spawn_Cue.Spawn_Cue" _returnvalue "0, 0, 0" 1.0 1.0 0.0 0 0 0)
                (Actor|DestroyActor)))))
        (:then_2
          (bind _returnvalue_2 (Utilities|Time|SetTimerbyEvent (delegate Custom|Rithm) 0.1 true))
          (Variables|Default|SetRithmTimer _returnvalue_2))))))

(fn ConstructionScript
  (|CallParentFunction))