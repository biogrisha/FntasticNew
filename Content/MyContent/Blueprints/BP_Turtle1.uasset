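; BP_Turtle1 is a turtle actor that, when activated, travels once along a referenced spline path and then vanishes.
; A slowed walking timeline maps its value to spline distance, setting location in world space and rotation in the spline's local space.
; A parallel acceleration timeline ramps Speed up, then reverses at the path's end.
; When that reversal finishes, the turtle spawns smoke, plays a sound and destroys itself.
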(event EventActivate
  (bind _returnvalue (Transformation|GetActorLocation))
  (bind _splinepath (Variables|Default|GetSplinePath))
  (bind _splinecomponent (Variables|/Game/MyContent/Blueprints/BP_SplinePath.BP_SplinePath_C|GetSplineComponent _splinepath))
  (Utilities|IsValid (Variables|Default|GetSplinePath)
    (:Is%20Valid
      (Components|Timeline|SetPlayRate (Variables|Default|GetWalkingTimeline) 0.2)
      (Utilities|FlowControl|Sequence
        (:then_0
          (bind _newtrack_0 (Timeline|WalkingTimeline PlayFromStart)
            (:Update
              (Transformation|SetActorTransform (Math|Transform|MakeTransform (Spline|GetLocationatDistanceAlongSpline _splinecomponent (* (Spline|GetSplineLength _splinecomponent) _newtrack_0) "World") (Spline|GetRotationatDistanceAlongSpline _splinecomponent (* (Spline|GetSplineLength _splinecomponent) _newtrack_0) "Local") "1,1,1")))
            (:Finished
              (bind (_direction _newtrack_0_2) (Timeline|AccelerationTimeline Reverse)
                (:Update
                  (Variables|Default|SetSpeed _newtrack_0_2))
                (:Finished
                  (if (Utilities|Enum|Equal(Enum) _direction "Backward")
                    (Effects|SpawnEmitteratLocation "/Game/MyContent/Assets/Effects/SmokeEffect.SmokeEffect" _returnvalue "0, 0, 0" "2.000000,2.000000,2.000000")
                    (Audio|PlaySoundatLocation "/Game/MyContent/Assets/Sounds/Spawn_Cue.Spawn_Cue" _returnvalue "0, 0, 0" 1.0 1.0 0.0 0 0 0)
                    (Actor|DestroyActor)))))))
        (:then_1
          (Timeline|AccelerationTimeline PlayFromStart))))))

(fn ConstructionScript
  (|CallParentFunction))